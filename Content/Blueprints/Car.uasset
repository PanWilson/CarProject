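; Car Blueprint that animates tire positions and steering from its custom suspension spring components.
; On BeginPlay it gathers the MySuspensionSpring components and the static meshes tagged Tire, pairing them by array index.
; Each Tick it offsets every tire vertically by spring height and flags front and back axle ground contact.
; The first two tires interpolate their yaw toward the maximum turn angle scaled by GetRotate.
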(event `self.ReceiveBeginPlay`
  (set `self.Suspensions` (`self.K2_GetComponentsByClass` "/Script/CarProject.MySuspensionSpring"))
  (set `self.Tires` (`self.GetComponentsByTag` "/Script/Engine.StaticMeshComponent" "Tire")))

(event `self.ReceiveTick`
  (params (DeltaSeconds :type "Float (single-precision)"))
  (bind _suspensions (`self.Suspensions`))
  (bind _suspensions_2 (`self.Suspensions`))
  (bind _tires (`self.Tires`))
  (bind (_relativerotation_roll _relativerotation_pitch _relativerotation_yaw) (`KismetMathLibrary.BreakRotator` (`SceneComponent.RelativeRotation` (`|GetArrayItem` _tires 1))))
  (for (_array_element _array_index) (`self.Tires`)
    (`SceneComponent.K2_SetRelativeLocation` _array_element (`KismetMathLibrary.MakeVector` 0.0 0.0 (* (`MySuspensionSpring.Height` (`|GetArrayItem` (`self.Suspensions`) _array_index)) -1.0)) false false))
  (`|ExecutionSequence`
    (:`then_0`
      (if (or (`MySuspensionSpring.OnGround` (`|GetArrayItem` _suspensions_2)) (`MySuspensionSpring.OnGround` (`|GetArrayItem` _suspensions_2 1)))
        (set `self.FrontAxelTouching` true)
        (else
          (set `self.FrontAxelTouching` false))))
    (:`then_1`
      (if (or (`MySuspensionSpring.OnGround` (`|GetArrayItem` _suspensions 2)) (`MySuspensionSpring.OnGround` (`|GetArrayItem` _suspensions 3)))
        (set `self.BackAxelTouching` true)
        (else
          (set `self.BackAxelTouching` false))))
    (:`then_2`
      (`SceneComponent.K2_SetRelativeRotation` (`|GetArrayItem` _tires) (`KismetMathLibrary.MakeRotator` _relativerotation_roll _relativerotation_pitch (`KismetMathLibrary.FInterpTo` _relativerotation_yaw (* (`self.MaxTurnDegre`) (`self.GetInputAxisValue`)) (`GameplayStatics.GetWorldDeltaSeconds`) 2.0)) false false)
      (`SceneComponent.K2_SetRelativeRotation` (`|GetArrayItem` _tires 1) (`KismetMathLibrary.MakeRotator` _relativerotation_roll _relativerotation_pitch (`KismetMathLibrary.FInterpTo` _relativerotation_yaw (* (`self.MaxTurnDegre`) (`self.GetInputAxisValue`)) (`GameplayStatics.GetWorldDeltaSeconds`) 2.0)) false false))))

(fn `UserConstructionScript`)